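; Tank pawn Blueprint that wires up the player's tank and its camera and firing controls.
; On BeginPlay it passes the turret and barrel components to the tank as references.
; Azimuth input yaws a gimbal and elevation input pitches the camera spring arm, orbiting the view on separate axes.
; The fire action calls FireCannon, whose logic lives outside these graphs.
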(event EventBeginPlay
  (Class|Tank|SetTurretReference (Variables|Default|GetTankTurret))
  (Class|Tank|SetBarrelReference (Variables|Default|GetTankBarrel)))

(event Collision|EventActorBeginOverlap
  (params (OtherActor :type Actor%20Object%20Reference)))

(event EventTick
  (params (DeltaSeconds :type Float%20%28single-precision%29)))

(event Input|ActionEvents|InputActionFireCannon
  (params (Key :type Key%20Structure))
  ;[1 1 1] Firing Controls
  (:Pressed
    (Class|Tank|FireCannon)))

(event Input|AxisEvents|InputAxisTurretAzimuth
  (params (AxisValue :type Float%20%28single-precision%29))
  ;[1 1 1] Camera Input Binding
  (Transformation|AddLocalRotation (Variables|Default|GetAzimuthGimble) (Math|Rotator|MakeRotator 0.0 0.0 AxisValue) false false))

(event Input|AxisEvents|InputAxisTurretElevation
  (params (AxisValue :type Float%20%28single-precision%29))
  ;[1 1 1] Camera Input Binding
  (Transformation|AddLocalRotation (Variables|Default|GetCameraSpringArm) (Math|Rotator|MakeRotator 0.0 AxisValue 0.0) false false))

(fn ConstructionScript)